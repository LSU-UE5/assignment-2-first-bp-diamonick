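; BP_Clock is a digital clock that shows the current time on a text component.
; Every Tick it reads Now, splits it into 12-hour hour, minute and second, and formats them as Hour:Minute:Second without an AM/PM marker.
; A helper function pads values below 10 with a leading zero.
; The construction script sets a 00:00:00 placeholder.
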(event EventTick
  (params (DeltaSeconds :type Float%20%28single-precision%29))
  ;[1 1 1 1 12] Format Text
  (bind _output_text (CallFunction|TimeFormatText(Int) (Class|KismetMathLibrary|GetSecond (Math|DateTime|Now))))
  (bind _output_text_2 (CallFunction|TimeFormatText(Int) (Class|KismetMathLibrary|GetMinute (Math|DateTime|Now))))
  (bind _output_text_3 (CallFunction|TimeFormatText(Int) (Class|KismetMathLibrary|GetHour12 (Math|DateTime|Now))))
  (Rendering|Components|TextRender|SetText (Variables|Default|GetTimeText) (Utilities|Text|FormatText "{Hour}:{Minute}:{Second}" _output_text_3 _output_text_2 _output_text)))

(fn ConstructionScript
  ;[1 1 1 1 12] Format Text
  (Rendering|Components|TextRender|SetText (Variables|Default|GetTimeText) (Utilities|Text|FormatText "00:00:00")))

(fn TimeFormatText(Int)
  (params (Value :type Integer))
  (bind _returnvalue (Utilities|Text|ToText(Integer) Value))
  ;[1 1 1] Check if value is < 10
  (if (< Value 10)
    ;[1 1 1] If integer is < 10, insert a "0" in front of the value
    (return (Utilities|Text|FormatText "0{A}" _returnvalue))
    (else
      ;[1 1 1] If integer is >= 10, print the value as it is.
      (return (Utilities|Text|FormatText _returnvalue)))))