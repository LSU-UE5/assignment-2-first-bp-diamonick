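; Blueprint for a guessing game where Space Bar presses count a guess up toward a hidden random number from 1 to 20.
; BeginPlay picks the number, and Tick compares it with the guess, showing the current count on a text render component.
; A match locks input and shows the win text, then a short Delay precedes a new random number and a zeroed guess.
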(event EventBeginPlay
  ;[1 1 1 1 12] Display random integer between 1 and 20
  (bind _output_get (Variables|Default|SetRandomInt (Math|Random|RandomIntegerinRange 1 20)))
  ;[1 1 1 1 12] Check if GuessInt equals RandomInt
  (if (== _output_get (Variables|Default|GetGuessInt))
    ;[1 1 1 1 12] Displays "You Win!" message
    (Rendering|Components|TextRender|SetText (Variables|Default|GetText%20Render) (Variables|Default|GetGuessText))
    ;[1 1 1 1 12] Reset Guessing Game
    (Utilities|FlowControl|Delay 2.0)
    (Variables|Default|SetRandomInt (Math|Random|RandomIntegerinRange 1 20))
    (Variables|Default|SetGuessInt 0)
    (else
      ;[1 1 1 1 12] Set Text
      (Rendering|Components|TextRender|SetText (Variables|Default|GetText%20Render) (Utilities|Text|ToText(Integer) (Variables|Default|GetGuessInt))))))

(event EventTick
  (params (DeltaSeconds :type Float%20%28single-precision%29))
  ;[1 1 1 1 12] Check if GuessInt equals RandomInt
  (if (== (stale EventBeginPlay _output_get) (Variables|Default|GetGuessInt))
    ;[1 1 1 1 12] Displays "You Win!" message
    (Rendering|Components|TextRender|SetText (Variables|Default|GetText%20Render) (Variables|Default|GetGuessText))
    ;[1 1 1 1 12] Reset Guessing Game
    (Utilities|FlowControl|Delay 2.0)
    (Variables|Default|SetRandomInt (Math|Random|RandomIntegerinRange 1 20))
    (Variables|Default|SetGuessInt 0)
    (else
      ;[1 1 1 1 12] Set Text
      (Rendering|Components|TextRender|SetText (Variables|Default|GetText%20Render) (Utilities|Text|ToText(Integer) (Variables|Default|GetGuessInt))))))

(event Input|KeyboardEvents|SpaceBar
  (params (Key :type Key%20Structure))
  ;[1 1 1 1 12] (Space Bar) Increment number
  (:Pressed
    (if (!= (Variables|Default|GetRandomInt) (Variables|Default|GetGuessInt))
      (Variables|Default|SetGuessInt (+ (Variables|Default|GetGuessInt) 1)))))

(fn ConstructionScript)